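; Game instance for a racing game that manages FMOD audio and race results across a multi-race gauntlet.
; On Init it loads the sound banks, and helper functions play one-shots, music and engine loops and set bus volumes and event parameters.
; StartRace enables driving; once seven finishers register, scores from a placement DataTable update totals and rankings.
; Racer structs are split into parallel arrays and rebuilt for partial updates.
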(event `self.ReceiveInit`
  (`self.InitBanks`))

(fn `AddFinishedPlayer`
  (params (Player :type "Pawn Object Reference") (Time :type "Timecode Structure"))
  (bind _finishedplayers (`self.FinishedPlayers`))
  (bind _finishtimes (`self.FinishTimes`))
  (`KismetArrayLibrary.Array_Add` _finishedplayers Player)
  (`KismetArrayLibrary.Array_Add` _finishtimes Time)
  (if (>= (`KismetArrayLibrary.Array_Length` _finishedplayers) 7)
    (`self.UpdateRacerArray` :`Time` _finishtimes)
    (`self.AddPointsToPlayer`)))

(fn `AddPointsToPlayer`
  (locals (NewScores :type "Array of Integer") (NewPlacements :type "Array of Byte") (SortedArray :type "Array of Integer") (NewLocalVar :type Integer))
  (bind _newscores (`local.NewScores`))
  (bind (_namesout _pawnsout) (`self.BreakRacerStrArray`))
  ;[1 1 1] add scores to each player
  (for (_array_element _array_index) (`self.FinishedPlayers`)
    (bind _outrownames (`DataTableFunctionLibrary.GetDataTableRowNames` "/Game/Blueprints/Gauntlet/DT_PlacementScoreRef.DT_PlacementScoreRef"))
    (bind _returnvalue (`|GetDataTableRow` "/Game/Blueprints/Gauntlet/DT_PlacementScoreRef.DT_PlacementScoreRef" (`|GetArrayItem` _outrownames _array_index))
      (:`then`
        (bind _returnvalue_2 (`KismetArrayLibrary.Array_Find` _pawnsout _array_element))
        (`KismetArrayLibrary.Array_Set` _newscores _returnvalue_2 (+ (`.GauntletScore_17_28DC8ADF49C02E7E7DFB759E2C9CB325` (break `/Game/Blueprints/Gauntlet/Str_Player` (`|GetArrayItem` (`self.Racers`) _returnvalue_2))) (`.GauntletScore_17_28DC8ADF49C02E7E7DFB759E2C9CB325` (break `/Game/Blueprints/Gauntlet/Str_Player` _returnvalue))) true))
      (:`RowNotFound`
        (`KismetArrayLibrary.Array_Set` _newscores _returnvalue_2 -1 true))))
  (bind _output_get (set `local.SortedArray` (`local.NewScores`)))
  (`KismetArrayLibrary.SortIntArray` _output_get false "Descending")
  (for (_array_element_2 _array_index_2) (`local.SortedArray`)
    (`KismetArrayLibrary.Array_Set` (`local.NewPlacements`) (`KismetArrayLibrary.Array_Find` (`local.NewScores`) _array_element_2) (`KismetMathLibrary.Conv_IntToByte` _array_index_2) true))
  (`self.UpdateRacerArray` :`Score` (`local.NewScores`) :`Placement` (`local.NewPlacements`)))

(fn `BreakRacerStrArray`
  (returns (NamesOUT :type "Array of String") (PawnsOUT :type "Array of Pawn Object Reference") (ScoresOUT :type "Array of Integer") (TimesOUT :type "Array of Timecode Structure") (PlacementsOUT :type "Array of Byte"))
  (locals (Names :type "Array of String") (Pawns :type "Array of Pawn Object Reference") (Scores :type "Array of Integer") (Times :type "Array of Timecode Structure") (Placements :type "Array of Byte"))
  (bind _racers (`self.Racers`))
  (for (_ _array_index) _racers
    (bind (_name _pawnreference _gauntletscore _currenttrackfinishtime _playerplacement) (break `/Game/Blueprints/Gauntlet/Str_Player` (`|GetArrayItem` _racers _array_index)))
    (`KismetArrayLibrary.Array_Set` (`local.Names`) _array_index _name true)
    (`KismetArrayLibrary.Array_Set` (`local.Pawns`) _array_index _pawnreference true)
    (`KismetArrayLibrary.Array_Set` (`local.Scores`) _array_index _gauntletscore true)
    (`KismetArrayLibrary.Array_Set` (`local.Times`) _array_index _currenttrackfinishtime true)
    (`KismetArrayLibrary.Array_Set` (`local.Placements`) _array_index _playerplacement true))
  (return (`local.Names`) (`local.Pawns`) (`local.Scores`) (`local.Times`) (`local.Placements`)))

(fn `InitBanks`
  (`FMODBlueprintStatics.LoadBank` "/Game/FMOD/Banks/Master.Master")
  (`FMODBlueprintStatics.LoadBank` "/Game/FMOD/Banks/AMBIENT.AMBIENT")
  (`FMODBlueprintStatics.LoadBank` "/Game/FMOD/Banks/BGM.BGM")
  (`FMODBlueprintStatics.LoadBank` "/Game/FMOD/Banks/FEEDBACK.FEEDBACK")
  (`FMODBlueprintStatics.LoadBank` "/Game/FMOD/Banks/ITEM.ITEM")
  (`FMODBlueprintStatics.LoadBank` "/Game/FMOD/Banks/LEVEL.LEVEL")
  (`FMODBlueprintStatics.LoadBank` "/Game/FMOD/Banks/MENU.MENU")
  (`FMODBlueprintStatics.LoadBank` "/Game/FMOD/Banks/NONPLAYER.NONPLAYER")
  (`FMODBlueprintStatics.LoadBank` "/Game/FMOD/Banks/PLAYER.PLAYER"))

(fn `Play One Shot`
  (params (Event :type "FMODEvent Object Reference") (Location :type "/Game/Blueprints/EAudioLocation Enum" :default "NewEnumerator0") (Transform :type "Transform Structure"))
  (returns (NewParam :type "FMODEventInstance Structure"))
  (switch `/Game/Blueprints/EAudioLocation` Location
    (:`NewEnumerator0`
      (`FMODBlueprintStatics.PlayEventAttached` Event null "None" (0.0 0.0 0.0) "KeepRelativeOffset"))
    (:`NewEnumerator1`
      (`FMODBlueprintStatics.PlayEventAtLocation` Event Transform)
      (return (stale _returnvalue)))
    (:`NewEnumerator2`
      (bind _returnvalue (`FMODBlueprintStatics.PlayEvent2D` Event))
      (return _returnvalue))))

(fn `PlayBGM`
  (params (Event :type "FMODEvent Object Reference") (StopImmediate :type Boolean))
  (if StopImmediate
    (`self.ReloadBank` "/Game/FMOD/Banks/BGM.BGM")
    (else
      (`FMODBlueprintStatics.EventInstanceStop` (`self.CurrentBGM`))))
  (bind _returnvalue (`FMODBlueprintStatics.PlayEvent2D` Event))
  (bind _output_get (set `self.CurrentBGM` _returnvalue))
  (`self.SetEventParameter` _output_get "IsGameStart"))

(fn `PlayEngine`
  (bind _returnvalue (`FMODBlueprintStatics.EventInstanceIsValid` (`self.CurrentEngine`)))
  (if _returnvalue
    (`self.SetEngineEvent` "/Game/FMOD/Events/SFX/VEHICLE/EngineLoop.EngineLoop")
    (else
      (`self.SetEngineEvent` "/Game/FMOD/Events/SFX/VEHICLE/EngineLoop.EngineLoop"))))

(fn `PlaySFXWithParameter`
  (params (Parameter :type Name) (Event :type "FMODEvent Object Reference") (Value :type "Float (double-precision)" :default 1.0))
  (bind _newparam (`self.Play One Shot` Event "NewEnumerator2"))
  (`self.SetEventParameter` _newparam Parameter Value))

(fn `ReloadBank`
  (params (Bank :type "FMODBank Object Reference"))
  (`FMODBlueprintStatics.UnloadBank` Bank)
  (`FMODBlueprintStatics.LoadBank` Bank))

(fn `SetBusVolume`
  (params (Bus :type "FMODBus Object Reference") (Volume :type "Float (double-precision)"))
  (`FMODBlueprintStatics.BusSetVolume` Bus Volume))

(fn `SetEngineEvent`
  (params (Event :type "FMODEvent Object Reference"))
  (bind _returnvalue (`FMODBlueprintStatics.PlayEvent2D` Event))
  (set `self.CurrentEngine` _returnvalue))

(fn `SetEventParameter`
  (params (Event :type "FMODEventInstance Structure") (Parameter :type Name) (Value :type "Float (double-precision)"))
  (`FMODBlueprintStatics.EventInstanceSetParameter` Event Parameter Value))

(fn `StartRace`
  (set `self.StartTimecode` (`TimeManagementBlueprintLibrary.GetTimecode`))
  (bind (_namesout _pawnsout) (`self.BreakRacerStrArray`))
  (for _array_element _pawnsout
    (bind _asbp_car (cast `/Game/Vehicles/BP_Car` _array_element))
    (set `/Game/Vehicles/BP_Car.CanDrive` true _asbp_car)))

(fn `StopBGM`
  (params (StopImmediate :type Boolean))
  (`FMODBlueprintStatics.EventInstanceStop` (`self.CurrentBGM`))
  (set `self.CurrentBGM` (struct)))

(fn `UpdateRacerArray`
  (params (Name :type "Array of String") (PawnRef :type "Array of Pawn Object Reference") (Score :type "Array of Integer") (Time :type "Array of Timecode Structure") (Placement :type "Array of Byte"))
  (locals (Names :type "Array of String") (Pawns :type "Array of Pawn Object Reference") (Scores :type "Array of Integer") (Times :type "Array of Timecode Structure") (Placements :type "Array of Byte"))
  (bind _racers (`self.Racers`))
  ;[1 1 1] create local var
  (bind _output_get (set `local.Names` Name))
  (bind _output_get_2 (set `local.Pawns` PawnRef))
  (bind _output_get_3 (set `local.Scores` Score))
  (bind _output_get_4 (set `local.Times` Time))
  (bind _output_get_5 (set `local.Placements` Placement))
  (bind _returnvalue (== (`KismetArrayLibrary.Array_Length` _output_get) 0))
  (bind _returnvalue_2 (== (`KismetArrayLibrary.Array_Length` _output_get_2) 0))
  (bind _returnvalue_3 (== (`KismetArrayLibrary.Array_Length` _output_get_3) 0))
  (bind _returnvalue_4 (== (`KismetArrayLibrary.Array_Length` _output_get_4) 0))
  (bind _returnvalue_5 (== (`KismetArrayLibrary.Array_Length` _output_get_5) 0))
  ;[1 1 1] throw if no array inputted
  (if (and _returnvalue _returnvalue_2 _returnvalue_3 _returnvalue_4 _returnvalue_5)
    (`KismetSystemLibrary.PrintString` "no information inputted for UpdateRacerArray")
    (else
      ;[1 1 1] for each array, if the inputted array is empty, copy contents of the Racers array into the local var
      (bind (_namesout _pawnsout _scoresout _timesout _placementsout) (`self.BreakRacerStrArray`))
      (if _returnvalue
        (set `local.Names` _namesout))
      (if _returnvalue_2
        (set `local.Pawns` _pawnsout))
      (if _returnvalue_3
        (set `local.Scores` _scoresout))
      (if _returnvalue_4
        (set `local.Times` _timesout))
      (if _returnvalue_5
        (set `local.Placements` _placementsout))
      ;[1 1 1] update racer array
      (for (_ _array_index) _racers
        (`KismetArrayLibrary.Array_Set` _racers _array_index (make `/Game/Blueprints/Gauntlet/Str_Player` (`|GetArrayItem` (`local.Names`) _array_index) (`|GetArrayItem` (`local.Pawns`) _array_index) (`|GetArrayItem` (`local.Scores`) _array_index) (`|GetArrayItem` (`local.Times`) _array_index) (`|GetArrayItem` (`local.Placements`) _array_index)))))))