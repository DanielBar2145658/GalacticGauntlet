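; FMOD audio manager that loads the game's sound banks on Init and centralises playback of music, effects and engine sounds.
; Helpers wrap bus volume, event parameters and one-shots played attached, at a location or in 2D.
; PlayBGM tracks the current instance and can cut music by reloading the BGM bank, while StopBGM's matching branch is unwired.
; PlayEngine starts the loop event if an engine instance is valid, otherwise the prerace event.
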(event `self.ReceiveInit`
  (`self.InitBanks`))

(fn `InitBanks`
  (`FMODBlueprintStatics.LoadBank` "/Game/FMOD/Banks/Master.Master")
  (`FMODBlueprintStatics.LoadBank` "/Game/FMOD/Banks/AMBIENT.AMBIENT")
  (`FMODBlueprintStatics.LoadBank` "/Game/FMOD/Banks/BGM.BGM")
  (`FMODBlueprintStatics.LoadBank` "/Game/FMOD/Banks/FEEDBACK.FEEDBACK")
  (`FMODBlueprintStatics.LoadBank` "/Game/FMOD/Banks/ITEM.ITEM")
  (`FMODBlueprintStatics.LoadBank` "/Game/FMOD/Banks/LEVEL.LEVEL")
  (`FMODBlueprintStatics.LoadBank` "/Game/FMOD/Banks/MENU.MENU")
  (`FMODBlueprintStatics.LoadBank` "/Game/FMOD/Banks/NONPLAYER.NONPLAYER")
  (`FMODBlueprintStatics.LoadBank` "/Game/FMOD/Banks/PLAYER.PLAYER"))

(fn `Play One Shot`
  (params (Event :type "FMODEvent Object Reference") (Location :type Byte :default 0) (Transform :type "Transform Structure"))
  (returns (NewParam :type "FMODEventInstance Structure"))
  (switch `|SwitchEnum` Location
    (:`NewEnumerator0`
      (`FMODBlueprintStatics.PlayEventAttached` Event null "None" (0.0 0.0 0.0) "KeepRelativeOffset"))
    (:`NewEnumerator1`
      (`FMODBlueprintStatics.PlayEventAtLocation` Event Transform)
      (return (stale _returnvalue)))
    (:`NewEnumerator2`
      (bind _returnvalue (`FMODBlueprintStatics.PlayEvent2D` Event))
      (return _returnvalue))))

(fn `PlayBGM`
  (params (Event :type "FMODEvent Object Reference") (StopImmediate :type Boolean))
  (if StopImmediate
    (`self.ReloadBank` "/Game/FMOD/Banks/BGM.BGM")
    (else
      (`FMODBlueprintStatics.EventInstanceStop` (`self.CurrentBGM`))))
  (bind _returnvalue (`FMODBlueprintStatics.PlayEvent2D` Event))
  (bind _output_get (set `self.CurrentBGM` _returnvalue))
  (`self.SetEventParameter` _output_get "IsGameStart"))

(fn `PlayEngine`
  (bind _returnvalue (`FMODBlueprintStatics.EventInstanceIsValid` (`self.CurrentEngine`)))
  (if _returnvalue
    (`self.SetEngineEvent` "/Game/FMOD/Events/SFX/VEHICLE/EngineLoop.EngineLoop")
    (else
      (`self.SetEngineEvent` "/Game/FMOD/Events/SFX/VEHICLE/EnginePrerace.EnginePrerace"))))

(fn `PlaySFXWithParameter`
  (params (Parameter :type Name) (Event :type "FMODEvent Object Reference") (Value :type "Float (double-precision)" :default 1.0))
  (bind _newparam (`self.Play One Shot` Event))
  (`self.SetEventParameter` _newparam Parameter Value))

(fn `ReloadBank`
  (params (Bank :type "FMODBank Object Reference"))
  (`FMODBlueprintStatics.UnloadBank` Bank)
  (`FMODBlueprintStatics.LoadBank` Bank))

(fn `SetBusVolume`
  (params (Bus :type "FMODBus Object Reference") (Volume :type "Float (double-precision)"))
  (`FMODBlueprintStatics.BusSetVolume` Bus Volume))

(fn `SetEngineEvent`
  (params (Event :type "FMODEvent Object Reference"))
  (bind _returnvalue (`FMODBlueprintStatics.PlayEvent2D` Event))
  (set `self.CurrentEngine` _returnvalue))

(fn `SetEventParameter`
  (params (Event :type "FMODEventInstance Structure") (Parameter :type Name) (Value :type "Float (double-precision)"))
  (`FMODBlueprintStatics.EventInstanceSetParameter` Event Parameter Value))

(fn `StopBGM`
  (params (StopImmediate :type Boolean))
  (`FMODBlueprintStatics.EventInstanceStop` (`self.CurrentBGM`))
  (set `self.CurrentBGM` (struct)))