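; BP_Item is the item held by a car in a racing-style game, tracking uses remaining and showing its graphic on the HUD.
; UseItem spends a use and switches on the item name to run its effect.
; Boost, Forcefield and Autopilot act on the owning BP_Car, while Asteroid, Lazer, EMP and Missle spawn actors at the owner, with Asteroid dropped behind.
; SetNewItem loads a new item and its uses after a guard check.
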(fn `Asteroid`
  (bind (_returnvalue_location _returnvalue_rotation) (`KismetMathLibrary.BreakTransform` (`Actor.GetTransform` (`self.GetOwner`))))
  (`|SpawnActorFromClass` "/Game/Blueprints/Items/Spawn/BP_ItemSpawn_Asteroid.BP_ItemSpawn_Asteroid_C" (`KismetMathLibrary.MakeTransform` (+ _returnvalue_location (* (`KismetMathLibrary.GetForwardVector` _returnvalue_rotation) -250.0)) _returnvalue_rotation) "Undefined" "MultiplyWithRoot" (`self.GetOwner`) null))

(fn `Autopilot`
  (bind _asbp_car (cast `/Game/Vehicles/BP_Car` (`self.GetOwner`)))
  (`/Game/Vehicles/BP_Car.AutopilotToggle` _asbp_car))

(fn `Boost`
  (bind _asbp_car (cast `/Game/Vehicles/BP_Car` (`self.GetOwner`)))
  (`/Game/Vehicles/BP_Car.Boost` _asbp_car 5.0 0.4))

(fn `DecrementItemUse`
  (set `self.UsesRemaining` (- (`self.UsesRemaining`) 1)))

(fn `EMP`
  (bind _returnvalue (`self.GetOwner`))
  (`|SpawnActorFromClass` "/Game/Blueprints/Items/Spawn/BP_ItemSpawn_EMP.BP_ItemSpawn_EMP_C" (`Actor.GetTransform` _returnvalue) "Undefined" "MultiplyWithRoot" _returnvalue null))

(fn `Forcefield`
  (bind _asbp_car (cast `/Game/Vehicles/BP_Car` (`self.GetOwner`)))
  (set `/Game/Vehicles/BP_Car.IsShield` true _asbp_car))

(fn `Lazer`
  (bind _returnvalue (`self.GetOwner`))
  (`|SpawnActorFromClass` "/Game/Blueprints/Items/Spawn/BP_ItemSpawn_Lazer.BP_ItemSpawn_Lazer_C" (`Actor.GetTransform` _returnvalue) "Undefined" "MultiplyWithRoot" _returnvalue null))

(fn `Missle`
  (bind _returnvalue (`self.GetOwner`))
  (`|SpawnActorFromClass` "/Game/Blueprints/Items/Spawn/BP_ItemSpawn_Missle.BP_ItemSpawn_Missle_C" (`Actor.GetTransform` _returnvalue) "Undefined" "MultiplyWithRoot" _returnvalue null))

(fn `SetItemUI`
  (params (NewParam :type "Texture2D Object Reference"))
  (bind _asnew_hud (cast `/Game/UI/NewHUD` (`PlayerController.GetHUD` (`GameplayStatics.GetPlayerController` 0)))
    (:`then`
      (`/Game/UI/BP_HUD.UpdateItemFrame` (`/Game/UI/NewHUD.UI_Reference` _asnew_hud) NewParam))
    (:`CastFailed`
      (`KismetSystemLibrary.PrintText` "failed to cast to HUD"))))

(fn `SetNewItem`
  (params (Item :type "/Game/Blueprints/Items/Str/Str_Item Structure"))
  (bind (_name _uses _item_graphic) (break `/Game/Blueprints/Items/Str/Str_Item` Item))
  (if (or (and (== (`.Name_11_F13660B54A24541F2B10C6B4A8408915` (break `/Game/Blueprints/Items/Str/Str_Item` (`self.Item`))) "Autopilot") (== (`self.UsesRemaining`) 0)) (< (`self.UsesRemaining`) 0))
    (`KismetSystemLibrary.PrintText` "Player Already Has Item")
    (else
      (set `self.Item` Item)
      (set `self.UsesRemaining` _uses)
      (`self.SetItemUI` _item_graphic)
      (`KismetSystemLibrary.PrintText` (`KismetTextLibrary.Conv_StringToText` (`KismetStringLibrary.Concat_StrStr` "Added " _name " with " (`KismetStringLibrary.Conv_ByteToString` _uses) " uses"))))))

(fn `UseItem`
  (if (> (`self.UsesRemaining`) 0)
    (`self.DecrementItemUse`)
    (`KismetSystemLibrary.PrintString` "Used Item")
    (switch `string` (`.Name_11_F13660B54A24541F2B10C6B4A8408915` (break `/Game/Blueprints/Items/Str/Str_Item` (`self.Item`)))
      (:`Boost`
        (`self.Boost`)
        (`self.SetItemUI` null :!label _label))
      (:`Asteroid`
        (`self.Asteroid`)
        (goto _label))
      (:`Lazer`
        (`self.Lazer`)
        (goto _label))
      (:`Forcefield`
        (`self.Forcefield`)
        (goto _label))
      (:`EMP`
        (`self.EMP`)
        (goto _label))
      (:`Missle`
        (`self.Missle`)
        (goto _label))
      (:`Autopilot`
        (`self.Autopilot`)))
    (else
      (`KismetSystemLibrary.PrintText` "No Item!"))))