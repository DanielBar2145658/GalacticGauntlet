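; BP_Item_1 is a racing item holder that stores a player's current item and its remaining uses.
; SetNewItem assigns an item after an already-has-item check, while UseItem spends a use and dispatches on the item name.
; Boost speeds up the player briefly; Forcefield, Asteroid, Lazer and EMP spawn item actors at the player's transform, with Forcefield also flagging the car shielded.
; Missle temporarily spawns the Lazer actor, and Autopilot is an empty stub.
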(fn `Asteroid`
  (`|SpawnActorFromClass` "/Game/Blueprints/Items/Spawn/BP_ItemSpawn_Asteroid.BP_ItemSpawn_Asteroid_C" (`Actor.GetTransform` (`self.PlayerRef`)) "Undefined" "MultiplyWithRoot" null null))

(fn `Autopilot`
  ;[1 1 1] i don't have this yet i do later
)

(fn `Boost`
  (bind _playerref (`self.PlayerRef`))
  (cast `Actor` _playerref)
  (`/Game/Vehicles/BP_Car.Boost` _playerref 5.0 0.4))

(fn `EMP`
  (`|SpawnActorFromClass` "/Game/Blueprints/Items/Spawn/BP_ItemSpawn_EMP.BP_ItemSpawn_EMP_C" (`Actor.GetTransform` (`self.PlayerRef`)) "Undefined" "MultiplyWithRoot" null null))

(fn `Forcefield`
  (bind _playerref (`self.PlayerRef`))
  (bind _asbp_car (cast `/Game/Vehicles/BP_Car` _playerref))
  (set `/Game/Vehicles/BP_Car.IsShield` true _asbp_car)
  (`|SpawnActorFromClass` "/Game/Blueprints/Items/Spawn/BP_ItemSpawn_ForceField.BP_ItemSpawn_ForceField_C" (`Actor.GetTransform` _playerref) "Undefined" "MultiplyWithRoot" null null))

(fn `Lazer`
  (`|SpawnActorFromClass` "/Game/Blueprints/Items/Spawn/BP_ItemSpawn_Lazer.BP_ItemSpawn_Lazer_C" (`Actor.GetTransform` (`self.PlayerRef`)) "Undefined" "MultiplyWithRoot" null null))

(fn `Missle`
  ;[1 1 1] i don't have this yet i do later
  (`|SpawnActorFromClass` "/Game/Blueprints/Items/Spawn/BP_ItemSpawn_Lazer.BP_ItemSpawn_Lazer_C" (`Actor.GetTransform` (`self.PlayerRef`)) "Undefined" "MultiplyWithRoot" null null))

(fn `SetNewItem`
  (params (Item :type "/Game/Blueprints/Items/Str/Str_Item Structure"))
  (bind (_name _uses) (break `/Game/Blueprints/Items/Str/Str_Item` Item))
  (if (or (not (== (`.Name_11_F13660B54A24541F2B10C6B4A8408915` (break `/Game/Blueprints/Items/Str/Str_Item` (`self.Item`))) "")) (> (`self.UsesRemaining`) 0))
    (`KismetSystemLibrary.PrintText` "Player Already Has Item")
    (else
      (set `self.Item` Item)
      (set `self.UsesRemaining` _uses)
      (`KismetSystemLibrary.PrintText` (`KismetTextLibrary.Conv_StringToText` (`KismetStringLibrary.Concat_StrStr` "Added " _name " with " (`KismetStringLibrary.Conv_ByteToString` _uses) " uses"))))))

(fn `UseItem`
  (bind _usesremaining (`self.UsesRemaining`))
  (if (> _usesremaining 0)
    (set `self.UsesRemaining` (- _usesremaining 1))
    (`KismetSystemLibrary.PrintString` "Used Item")
    (switch `string` (`.Name_11_F13660B54A24541F2B10C6B4A8408915` (break `/Game/Blueprints/Items/Str/Str_Item` (`self.Item`)))
      (:`Boost`
        (`self.Boost`))
      (:`Asteroid`
        (`self.Asteroid`))
      (:`Lazer`
        (`self.Lazer`))
      (:`Forcefield`
        (`self.Forcefield`))
      (:`EMP`
        (`self.EMP`))
      (:`Missle`
        (`self.Missle`))
      (:`Autopilot`
        (`self.Autopilot`)))))