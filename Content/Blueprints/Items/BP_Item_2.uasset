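; Item handler owned by a car that holds one item with limited uses and activates its effect.
; SetNewItem accepts an item only when no uses remain, while UseItem spends a use and dispatches on the item name.
; Boost calls BP_Car, Forcefield sets its shield flag and spawns an actor, and Asteroid, Lazer and EMP spawn actors at the owner's transform.
; Both update the HUD item frame; Missle and Autopilot are empty stubs.
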(fn `Asteroid`
  (`|SpawnActorFromClass` "/Game/Blueprints/Items/Spawn/BP_ItemSpawn_Asteroid.BP_ItemSpawn_Asteroid_C" (`Actor.GetTransform` (`self.GetOwner`)) "Undefined" "MultiplyWithRoot" null null))

(fn `Autopilot`)

(fn `Boost`
  (bind _asbp_car (cast `/Game/Vehicles/BP_Car` (`self.GetOwner`)))
  (`/Game/Vehicles/BP_Car.Boost` _asbp_car 5.0 0.4))

(fn `EMP`
  (`|SpawnActorFromClass` "/Game/Blueprints/Items/Spawn/BP_ItemSpawn_EMP.BP_ItemSpawn_EMP_C" (`Actor.GetTransform` (`self.GetOwner`)) "Undefined" "MultiplyWithRoot" null null))

(fn `Forcefield`
  (bind _returnvalue (`self.GetOwner`))
  (bind _asbp_car (cast `/Game/Vehicles/BP_Car` _returnvalue))
  (set `/Game/Vehicles/BP_Car.IsShield` true _asbp_car)
  (`|SpawnActorFromClass` null (`Actor.GetTransform` _returnvalue) "Undefined" "MultiplyWithRoot" null null))

(fn `Lazer`
  (`|SpawnActorFromClass` "/Game/Blueprints/Items/Spawn/BP_ItemSpawn_Lazer.BP_ItemSpawn_Lazer_C" (`Actor.GetTransform` (`self.GetOwner`)) "Undefined" "MultiplyWithRoot" null null))

(fn `Missle`)

(fn `SetItemUI`
  (params (NewParam :type "Texture2D Object Reference"))
  (bind _asnew_hud (cast `/Game/UI/NewHUD` (`PlayerController.GetHUD` (`GameplayStatics.GetPlayerController` 0)))
    (:`then`
      (`/Game/UI/BP_HUD.UpdateItemFrame` (`/Game/UI/NewHUD.UI_Reference` _asnew_hud) NewParam))
    (:`CastFailed`
      (`KismetSystemLibrary.PrintText` "failed to cast to HUD"))))

(fn `SetNewItem`
  (params (Item :type "/Game/Blueprints/Items/Str/Str_Item Structure"))
  (bind (_name _uses _item_graphic) (break `/Game/Blueprints/Items/Str/Str_Item` Item))
  (if (or false (> (`self.UsesRemaining`) 0))
    (`KismetSystemLibrary.PrintText` "Player Already Has Item")
    (else
      (set `self.Item` Item)
      (set `self.UsesRemaining` _uses)
      (`self.SetItemUI` _item_graphic)
      (`KismetSystemLibrary.PrintText` (`KismetTextLibrary.Conv_StringToText` (`KismetStringLibrary.Concat_StrStr` "Added " _name " with " (`KismetStringLibrary.Conv_ByteToString` _uses) " uses"))))))

(fn `UseItem`
  (bind _usesremaining (`self.UsesRemaining`))
  (if (> _usesremaining 0)
    (set `self.UsesRemaining` (- _usesremaining 1))
    (`KismetSystemLibrary.PrintString` "Used Item")
    (`self.SetItemUI` null)
    (switch `string` (`.Name_11_F13660B54A24541F2B10C6B4A8408915` (break `/Game/Blueprints/Items/Str/Str_Item` (`self.Item`)))
      (:`Boost`
        (`self.Boost`))
      (:`Asteroid`
        (`self.Asteroid`))
      (:`Lazer`
        (`self.Lazer`))
      (:`Forcefield`
        (`self.Forcefield`))
      (:`EMP`
        (`self.EMP`))
      (:`Missle`
        (`self.Missle`))
      (:`Autopilot`
        (`self.Autopilot`)))
    (else
      (`KismetSystemLibrary.PrintText` "No Item!"))))