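; Racing item missile that seeks the car in first place and damages the first valid "canDamage" actor it overlaps, then destroys itself.
; Construction picks the target from the game instance's racer list, finds the track spline and starts a timer that later allows hitting the owner.
; Tick steers along the spline by input key, then switches permanently to direct homing once on the spline and within range of an allowed target.
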(event `self.ReceiveBeginPlay`)

(event `self.ReceiveTick`
  (params (DeltaSeconds :type "Float (single-precision)"))
  (if (`self.HomingPlayer`)
    (`self.NavHomingPlayer` DeltaSeconds)
    (else
      (`self.NavToSpline` DeltaSeconds))))

(event `self.ReceiveActorBeginOverlap`
  (params (OtherActor :type "Actor Object Reference"))
  ;[1 1 1] Check if collision is with car or debug damage object AND the object is not the player that shot the object
  (if (and (`self.ActorHasTag` OtherActor "canDamage") (or (`self.canHitOwner`) (!= OtherActor (`self.GetOwner`))))
    (`GameplayStatics.ApplyDamage` OtherActor 3.0)
    (`self.K2_DestroyActor`)
    (else
      (`KismetSystemLibrary.PrintString` (`KismetStringLibrary.Concat_StrStr` "missile contact:" (`KismetStringLibrary.Conv_ObjectToString` OtherActor))))))

(fn `IsNearSpline`
  (returns (IsNear :type Boolean))
  (bind _returnvalue (< (`KismetMathLibrary.Vector_Distance` (`SplineComponent.GetLocationAtSplineInputKey` (`/Game/Placeables/Laps/BP_TrackSpline.Spline` (`self.Track`)) (`self.CurrentSplineKey`) "World") (`self.K2_GetActorLocation`)) (`self.DistanceForAlong`)))
  (if _returnvalue
    (set `self.OnSpline` true))
  (return _returnvalue))

(fn `NavHomingPlayer`
  (params (deltaTime :type "Float (double-precision)"))
  (`self.K2_AddActorWorldOffset` (* (`KismetMathLibrary.GetDirectionUnitVector` (`self.K2_GetActorLocation`) (`self.K2_GetActorLocation` (`self.TargetPlayer`))) (* deltaTime (`self.Speed`)))))

(fn `NavToSpline`
  (params (deltaTime :type "Float (double-precision)"))
  (`self.IsNearSpline`)
  (if (`self.OnSpline`)
    (`self.ResetSplineKey`))
  (set `self.CurrentSplineKey` (+ (`self.CurrentSplineKey`) deltaTime))
  (`self.K2_AddActorWorldOffset` (* (`KismetMathLibrary.GetDirectionUnitVector` (`self.K2_GetActorLocation`) (`SplineComponent.GetLocationAtSplineInputKey` (`/Game/Placeables/Laps/BP_TrackSpline.Spline` (`self.Track`)) (`self.CurrentSplineKey`) "World")) (* deltaTime (`self.Speed`))))
  (if (and (<= (`KismetMathLibrary.Vector_Distance` (`self.K2_GetActorLocation`) (`self.K2_GetActorLocation` (`self.TargetPlayer`))) (`self.DistanceToHoming`)) (`self.OnSpline`))
    (if (or (!= (`self.GetOwner`) (`self.TargetPlayer`)) (`self.canHitOwner`))
      (set `self.HomingPlayer` true))))

(fn `OwnerTimer`
  (set `self.canHitOwner` true))

(fn `ResetSplineKey`
  (set `self.CurrentSplineKey` (`SplineComponent.FindInputKeyClosestToWorldLocation` (`/Game/Placeables/Laps/BP_TrackSpline.Spline` (`self.Track`)) (`self.K2_GetActorLocation`))))

(fn `SetTarget`
  (bind _asgi_racing_manager (cast `/Game/Blueprints/GI_RacingManager` (`GameplayStatics.GetGameInstance`)))
  (for _array_element (`/Game/Blueprints/GI_RacingManager.Racers` _asgi_racing_manager)
    (bind (_name _pawnreference) (break `/Game/Blueprints/Gauntlet/Player/Str_Player` _array_element))
    (bind _asbp_car (cast `/Game/Vehicles/BP_Car` _pawnreference))
    (if (== (`/Game/Vehicles/BP_Car.Placement` _asbp_car) 1)
      (set `self.TargetPlayer` _pawnreference)
      (break))))

(fn `UserConstructionScript`
  (`self.SetTarget`)
  (cast `/Game/Blueprints/GI_RacingManager` (`GameplayStatics.GetGameInstance`))
  (bind _returnvalue (`GameplayStatics.GetActorOfClass` "/Game/Placeables/Laps/BP_TrackSpline.BP_TrackSpline_C"))
  (set `self.Track` _returnvalue)
  (`self.ResetSplineKey`)
  (`KismetSystemLibrary.K2_SetTimer` null "OwnerTimer" (`self.canHitTimer`)))