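; EMP item spawn actor that acts as a temporary damage source for actors that overlap it.
; BeginPlay computes an end time from the Lifetime variable, and Tick destroys the actor once game time passes it.
; Any actor that begins overlapping receives a small fixed amount of damage, with no filtering by type or owner.
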(event `self.ReceiveBeginPlay`
  (set `self.EndTime` (+ (`GameplayStatics.GetTimeSeconds`) (`self.Lifetime`))))

(event `self.ReceiveTick`
  (params (DeltaSeconds :type "Float (single-precision)"))
  (if (> (`GameplayStatics.GetTimeSeconds`) (`self.EndTime`))
    (`self.K2_DestroyActor`)))

(event `self.ReceiveActorBeginOverlap`
  (params (OtherActor :type "Actor Object Reference"))
  (`GameplayStatics.ApplyDamage` OtherActor 1.0))

(fn `UserConstructionScript`)