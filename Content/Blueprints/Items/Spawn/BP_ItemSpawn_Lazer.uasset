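; BP_ItemSpawn_Lazer is a laser projectile spawned by an item, fired by a player at cars and other damageable objects.
; Tick moves it forward along its rotation at a set speed without sweeping and destroys it once its lifetime expires.
; On overlap it damages any actor tagged canDamage other than its owner and destroys itself, otherwise it prints the contact for debugging.
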(event `self.ReceiveBeginPlay`
  (set `self.EndTime` (+ (`GameplayStatics.GetTimeSeconds`) (`self.Lifetime`))))

(event `self.ReceiveTick`
  (params (DeltaSeconds :type "Float (single-precision)"))
  (if (> (`GameplayStatics.GetTimeSeconds`) (`self.EndTime`))
    (`self.K2_DestroyActor`)
    (else
      (`self.K2_AddActorWorldOffset` (* DeltaSeconds (`KismetMathLibrary.GetForwardVector` (`self.K2_GetActorRotation`)) (`self.Speed`))))))

(event `self.ReceiveActorBeginOverlap`
  (params (OtherActor :type "Actor Object Reference"))
  ;[1 1 1] Check if collision is with car or debug damage object AND the object is not the player that shot the object
  (if (and (`self.ActorHasTag` OtherActor "canDamage") (!= OtherActor (`self.GetOwner`)))
    (`GameplayStatics.ApplyDamage` OtherActor 2.0)
    (`self.K2_DestroyActor`)
    (else
      (`KismetSystemLibrary.PrintString` (`KismetStringLibrary.Concat_StrStr` "lazer contact: " (`KismetStringLibrary.Conv_ObjectToString` OtherActor))))))

(fn `UserConstructionScript`)