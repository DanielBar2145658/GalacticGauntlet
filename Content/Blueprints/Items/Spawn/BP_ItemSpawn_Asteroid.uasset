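; Spawned asteroid item that spins in place and damages actors tagged "canDamage" on overlap, then destroys itself.
; The construction script randomly keeps one of three asteroid components, destroys the others and starts a short timer to enable CanDamage.
; Until that timer calls AllowDamage, the overlap check excludes the actor's owner, while other tagged actors can be hit immediately.
; Tick applies the local rotation, scaled by RotationSpeed and frame time.
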(event `self.ReceiveTick`
  (params (DeltaSeconds :type "Float (single-precision)"))
  (`self.K2_AddActorLocalRotation` (* (struct :`Yaw` 1.0) (* DeltaSeconds (`self.rotationSpeed`)))))

(event `self.ReceiveActorBeginOverlap`
  (params (OtherActor :type "Actor Object Reference"))
  (if (and (`self.ActorHasTag` OtherActor "canDamage") (or (!= OtherActor (`self.GetOwner`)) (`self.canDamage`)))
    (`GameplayStatics.ApplyDamage` OtherActor 3.0)
    (`self.K2_DestroyActor`)))

(fn `AllowDamage`
  (set `self.canDamage` true))

(fn `UserConstructionScript`
  (bind _ggasteroid2sharpened__1_ (`self.GGAsteroid2Sharpened__1_`))
  (bind _ggasteroid3sharpened__1_ (`self.GGAsteroid3Sharpened__1_`))
  (bind _ggasteroid1sharpened__1_ (`self.GGAsteroid1Sharpened__1_`))
  ;[1 1 1] use a random asteroid; delete the unused asteroids
  (switch `int` (`KismetMathLibrary.RandomIntegerInRange` 0 2)
    (:`0`
      (`ActorComponent.K2_DestroyComponent` _ggasteroid2sharpened__1_)
      (`ActorComponent.K2_DestroyComponent` _ggasteroid3sharpened__1_))
    (:`1`
      (`ActorComponent.K2_DestroyComponent` _ggasteroid1sharpened__1_)
      (`ActorComponent.K2_DestroyComponent` _ggasteroid3sharpened__1_))
    (:`2`
      (`ActorComponent.K2_DestroyComponent` _ggasteroid1sharpened__1_)
      (`ActorComponent.K2_DestroyComponent` _ggasteroid2sharpened__1_)))
  (`KismetSystemLibrary.K2_SetTimer` null "AllowDamage" 0.5))