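; Player-driven arcade racing car pawn with items, shield, tiered damage slowdowns and drift-charged speed boosts.
; Each tick, four raycast suspensions push the physics Box up and forward using AccelerationInput and data-asset engine stats; a flight state uses direct thrust and rotation.
; Timed autopilot steers along the BP_TrackSpline via look-ahead dot products.
; GI_RacingManager handles racer registration, audio and saved location; debug keys spawn AI, grant items and change materials.
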(event OnComponentBeginOverlap(Box)
  (params (OverlappedComponent :type Primitive%20Component%20Object%20Reference) (OtherActor :type Actor%20Object%20Reference) (OtherComp :type Primitive%20Component%20Object%20Reference) (OtherBodyIndex :type Integer) (bFromSweep :type Boolean) (SweepResult :type Hit%20Result%20Structure%20%28by%20ref%29))
  (bind _asbp_gravity_affector (Utilities|Casting|CastToBP_GravityAffector OtherActor))
  (bind _newparam (Default|GetGravityDirection _asbp_gravity_affector self))
  (Transformation|AddLocalRotation (Variables|Default|GetBox) (Math|Conversions|RotationFromXVector _newparam) false false))

(event OnComponentBeginOverlap(Box2)
  (params (OverlappedComponent :type Primitive%20Component%20Object%20Reference) (OtherActor :type Actor%20Object%20Reference) (OtherComp :type Primitive%20Component%20Object%20Reference) (OtherBodyIndex :type Integer) (bFromSweep :type Boolean) (SweepResult :type Hit%20Result%20Structure%20%28by%20ref%29))
  (bind _asbp_car (Utilities|Casting|CastToBP_Car OtherActor))
  (CallFunction|CollisionPush _asbp_car (* (Class|KismetMathLibrary|VectorRight) "0.000000,500.000000,0.000000")))

(event OnComponentBeginOverlap(Box1)
  (params (OverlappedComponent :type Primitive%20Component%20Object%20Reference) (OtherActor :type Actor%20Object%20Reference) (OtherComp :type Primitive%20Component%20Object%20Reference) (OtherBodyIndex :type Integer) (bFromSweep :type Boolean) (SweepResult :type Hit%20Result%20Structure%20%28by%20ref%29))
  (bind _asbp_car (Utilities|Casting|CastToBP_Car OtherActor))
  (CallFunction|CollisionPush _asbp_car (* (Class|KismetMathLibrary|VectorRight) "0.000000,-500.000000,0.000000")))

(event Input|EnhancedActionEvents|EnhancedInputActionIA_Accelerate
  (params (ActionValue :type Boolean) (ElapsedSeconds :type Float%20%28double-precision%29) (TriggeredSeconds :type Float%20%28double-precision%29) (InputAction :type Input%20Action%20Object%20Reference :default "/Game/InputMapping/InputActions/IA_Accelerate.IA_Accelerate"))
  (if (Variables|Default|GetCanDrive)
    (Variables|Default|SetAccelerationInput (Math|Interpolation|FInterpTo (Variables|Default|GetAccelerationInput) 1.0 (Utilities|Time|GetWorldDeltaSeconds) 0.2))))

(event Input|EnhancedActionEvents|EnhancedInputActionIA_Steer
  (params (ActionValue :type Vector%202D%20Structure) (ElapsedSeconds :type Float%20%28double-precision%29) (TriggeredSeconds :type Float%20%28double-precision%29) (InputAction :type Input%20Action%20Object%20Reference :default "/Game/InputMapping/InputActions/IA_Steer.IA_Steer"))
  (bind (_x _y) (Math|Vector2D|BreakVector2D ActionValue))
  (if (Variables|Default|GetCanDrive)
    (if (Utilities|Enum|Equal(Enum) (Variables|Default|GetVehicle%20State) "NewEnumerator0")
      (Class|PrimitiveComponent|AddTorqueinRadians (Variables|Default|GetBox) (Math|Vector|MakeVector 0.0 0.0 (* (* _x (Variables|Default|GetHandling) (Variables|Default|GetAccelerationInput)) (Variables|Default|GetDriftFact))) "None" false)
      (else
        (Transformation|AddLocalRotation (Variables|Default|GetBox) (Math|Rotator|MakeRotator 0.0 (Math|Float|Lerp 0.0 (* _y (Variables|Default|GetHandlin_Air) (Variables|Default|GetAccelerationInput) (Variables|Default|GetInverted)) 0.5) (Math|Float|Lerp 0.0 (* _x (Variables|Default|GetHandlin_Air) 0.55) 0.5)) false false)))))

(event Input|EnhancedActionEvents|EnhancedInputActionIA_Drift
  (params (ActionValue :type Boolean) (ElapsedSeconds :type Float%20%28double-precision%29) (TriggeredSeconds :type Float%20%28double-precision%29) (InputAction :type Input%20Action%20Object%20Reference :default "/Game/InputMapping/InputActions/IA_Drift.IA_Drift"))
  (:Ongoing
    (if (Variables|Default|GetCanDrive)
      (CallFunction|Drift 0.0 false (.X (Math|Vector2D|BreakVector2D (stale Input|EnhancedActionEvents|EnhancedInputActionIA_Steer ActionValue))))
      (Development|PrintString "Drifting")))
  (:Completed
    (Variables|Default|SetIsDrifting false)
    (Variables|Default|SetDriftFact 1.0)
    (CallFunction|DriftBoost (Variables|Default|GetBoost%20Level))
    (Variables|Default|SetBoost%20Level 0)))

(event Input|EnhancedActionEvents|EnhancedInputActionIA_LoadLocation
  (params (ActionValue :type Boolean) (ElapsedSeconds :type Float%20%28double-precision%29) (TriggeredSeconds :type Float%20%28double-precision%29) (InputAction :type Input%20Action%20Object%20Reference :default "/Game/InputMapping/InputActions/Debug/IA_LoadLocation.IA_LoadLocation"))
  (bind _asgi_racing_manager (Utilities|Casting|CastToGI_RacingManager (Game|GetGameInstance)))
  (Transformation|SetActorTransform (Variables|/Game/Blueprints/GI_RacingManager.GI_RacingManager_C|GetLastKnownLocation _asgi_racing_manager) false true))

(event Input|EnhancedActionEvents|EnhancedInputActionIA_SaveLocation
  (params (ActionValue :type Boolean) (ElapsedSeconds :type Float%20%28double-precision%29) (TriggeredSeconds :type Float%20%28double-precision%29) (InputAction :type Input%20Action%20Object%20Reference :default "/Game/InputMapping/InputActions/Debug/IA_SaveLocation.IA_SaveLocation"))
  (bind _asgi_racing_manager (Utilities|Casting|CastToGI_RacingManager (Game|GetGameInstance)))
  (Variables|/Game/Blueprints/GI_RacingManager.GI_RacingManager_C|SetLastKnownLocation _asgi_racing_manager (Transformation|GetWorldTransform (Variables|Default|GetBox))))

(event Input|EnhancedActionEvents|EnhancedInputActionIA_UseItem
  (params (ActionValue :type Boolean) (ElapsedSeconds :type Float%20%28double-precision%29) (TriggeredSeconds :type Float%20%28double-precision%29) (InputAction :type Input%20Action%20Object%20Reference :default "/Game/InputMapping/InputActions/IA_UseItem.IA_UseItem"))
  (Default|UseItem (Variables|Default|GetBP_Item)))

(event Input|EnhancedActionEvents|EnhancedInputActionIA_Brake
  (params (ActionValue :type Boolean) (ElapsedSeconds :type Float%20%28double-precision%29) (TriggeredSeconds :type Float%20%28double-precision%29) (InputAction :type Input%20Action%20Object%20Reference :default "/Game/InputMapping/InputActions/IA_Brake.IA_Brake"))
  (if (Variables|Default|GetCanDrive)
    (if (> (Variables|Default|GetAccelerationInput) 0.0)
      (Variables|Default|SetAccelerationInput (Math|Interpolation|FInterpTo (Variables|Default|GetAccelerationInput) 0.0 (Utilities|Time|GetWorldDeltaSeconds) 0.0))
      (else
        (Variables|Default|SetAccelerationInput (Math|Interpolation|FInterpTo (Variables|Default|GetAccelerationInput) -0.5 (Utilities|Time|GetWorldDeltaSeconds) 0.2))))))

(event EventBeginPlay
  (Utilities|FlowControl|Delay 0.2)
  ;[0.1928 1 0] Casting Player Controller
  (bind _asplayer_controller (Utilities|Casting|CastToPlayerController (Pawn|GetController)))
  (Input|AddMappingContext (PlayerController|LocalPlayerSubsystems|GetEnhancedInputLocalPlayerSubsystem _asplayer_controller) "/Game/InputMapping/IA_Player.IA_Player" 0 "(bIgnoreAllPressedKeysUntilRelease=True,bForceImmediately=False,bNotifyUserSettings=False)")
  (Components|Activation|Deactivate (Variables|Default|GetSpeedVFX))
  (bind _asgi_racing_manager (Utilities|Casting|CastToGI_RacingManager (Game|GetGameInstance)))
  (bind _returnvalue (Actor|GetActorOfClass "/Game/Placeables/Laps/BP_TrackSpline.BP_TrackSpline_C"))
  (Variables|Default|SetTrack _returnvalue)
  (Utilities|Array|Add (Variables|/Game/Blueprints/GI_RacingManager.GI_RacingManager_C|GetRacers _asgi_racing_manager) self)
  (Development|PrintString "Added To Racer")
  ;[1 1 1] remove this later when i actually properly implement this -x
  (Default|PlayEngine _asgi_racing_manager))

(event Game|Damage|EventAnyDamage
  (params (Damage :type Float%20%28single-precision%29) (DamageType :type Damage%20Type%20Object%20Reference) (InstigatedBy :type Controller%20Object%20Reference) (DamageCauser :type Actor%20Object%20Reference))
  (if (Variables|Default|GetIsShield)
    (Variables|Default|SetIsShield false)
    (else
      (CallFunction|Damage (Math|Float|Truncate Damage)))))

(event EventTick
  (params (DeltaSeconds :type Float%20%28single-precision%29))
  (if (Variables|Default|GetIsAutopilot)
    (CallFunction|Autopilot))
  (if (Utilities|Enum|Equal(Enum) (Variables|Default|GetVehicle%20State) "NewEnumerator0")
    ;[0.763 0.09722 1] Set Suspensions on Vehicel
    (CallFunction|BindSuspensions DeltaSeconds)
    (CallFunction|CalculateAcceleration)
    (else
      (CallFunction|FlightControls)
      (CallFunction|CalculateAcceleration)
      (Variables|Default|SetA (Transformation|GetWorldRotation (Variables|Default|GetBox))))))

(event Collision|EventActorBeginOverlap
  (params (OtherActor :type Actor%20Object%20Reference)))

(event Input|KeyboardEvents|DebugKeyT
  (params (Key :type Key%20Structure) (ActionValue :type Input%20Action%20Value%20Structure))
  (:Pressed
    (bind _asgi_racing_manager (Utilities|Casting|CastToGI_RacingManager (Game|GetGameInstance)))
    (Rendering|Material|SetMaterial (Variables|Default|GetCube) 0 (Utilities|Array|Get(acopy) (.material (Variables|/Game/Blueprints/GI_RacingManager.GI_RacingManager_C|GetCarStats _asgi_racing_manager)) (Variables|Default|GetCurretnMaterial)))
    (Variables|Default|SetCurretnMaterial (+ (Variables|Default|GetCurretnMaterial) 1))
    (if (>= 0 (Utilities|Array|Length (.material (Variables|/Game/Blueprints/GI_RacingManager.GI_RacingManager_C|GetCarStats _asgi_racing_manager))))
      (Variables|Default|SetCurretnMaterial 0)
      (else
        (Development|PrintString "Changed Material")))))

(event Input|KeyboardEvents|DebugKeyJ
  (params (Key :type Key%20Structure) (ActionValue :type Input%20Action%20Value%20Structure))
  (:Pressed
    (Game|SpawnActorfromClass "/Game/Vehicles/BP_AICar.BP_AICar_C" (Math|Transform|MakeTransform (+ (.location (Transformation|GetWorldTransform (Variables|Default|GetBox))) "10.000000,0.000000,20.000000")) "Undefined" "MultiplyWithRoot" 0 0)
    (Development|PrintString "AISPawned")))

(event Input|KeyboardEvents|DebugKeyU
  (params (Key :type Key%20Structure) (ActionValue :type Input%20Action%20Value%20Structure))
  (bind _returnvalue (Game|GetPlayerController 0))
  (bind _returnvalue_2 (Game|GetPlayerController 0))
  (:Pressed
    (Utilities|IsValid (Variables|Default|GetRef_Settings)
      (:Is%20Valid
        (if (Widget|IsVisible (Variables|Default|GetRef_Settings))
          (Input|SetInputModeGameOnly _returnvalue_2 false)
          (Variables|/Script/Engine.PlayerController|SetbShowMouseCursor _returnvalue_2 false)
          (else
            (UserInterface|Viewport|AddtoViewport (stale _output_get) 0 :!label _label)
            (Input|SetInputModeGameandUI _returnvalue 0 "DoNotLock" false false)
            (Variables|/Script/Engine.PlayerController|SetbShowMouseCursor _returnvalue true))))
      (:Is%20Not%20Valid
        (bind _returnvalue_3 (UserInterface|CreateWidget "/Game/UI/DebugMenu/WI_Debug.WI_Debug_C"))
        (bind _output_get (Variables|Default|SetRef_Settings _returnvalue_3))
        (goto _label)))))

(event Input|KeyboardEvents|DebugKeyR
  (params (Key :type Key%20Structure) (ActionValue :type Input%20Action%20Value%20Structure))
  (:Pressed
    (Transformation|SetActorTransform (Math|Transform|MakeTransform (Transformation|GetActorLocation) (Math|Rotator|MakeRotator 0.0 0.0 (.yaw (Transformation|GetActorRotation)))))))

(event Input|KeyboardEvents|DebugKey0
  (params (Key :type Key%20Structure) (ActionValue :type Input%20Action%20Value%20Structure))
  (:Pressed
    (bind _asgi_racing_manager (Utilities|Casting|CastToGI_RacingManager (Game|GetGameInstance)))
    (Default|PlayBGM _asgi_racing_manager "/Game/FMOD/Events/BGM/LEVEL/Moon/BGM.BGM" false)))

(event Input|KeyboardEvents|DebugKeyI
  (params (Key :type Key%20Structure) (ActionValue :type Input%20Action%20Value%20Structure))
  (:Pressed
    (bind _outrownames (DataTable|GetDataTableRowNames "/Game/Blueprints/Items/Str/DT_ItemTable.DT_ItemTable"))
    (bind _returnvalue (Utilities|GetDataTableRow "/Game/Blueprints/Items/Str/DT_ItemTable.DT_ItemTable" (Utilities|Array|Get(acopy) _outrownames (Math|Random|RandomInteger (Utilities|Array|Length _outrownames))))
      (:then
        (CallFunction|SetItem _returnvalue)
        (Development|PrintText (Utilities|Text|ToText(String) (Utilities|String|Append "Got Item: " (.Name (Utilities|Struct|BreakStr_Item _returnvalue))))))
      (:RowNotFound
        (Development|PrintText "Invalid Item?")))))

(event Input|KeyboardEvents|DebugKeyN
  (params (Key :type Key%20Structure) (ActionValue :type Input%20Action%20Value%20Structure))
  (:Pressed
    (CallFunction|AutopilotToggle)))

(event Input|KeyboardEvents|AnyKey
  (params (Key :type Key%20Structure))
  (bind _returnvalue (Class|KismetInputLibrary|KeyGetDisplayName Key false))
  (bind _returnvalue_2 (Utilities|String|ToString(Text) _returnvalue))
  (bind _returnvalue_3 (Math|Conversions|ToInteger(Byte) _returnvalue_2))
  (:Pressed
    (bind _outrownames (DataTable|GetDataTableRowNames "/Game/Blueprints/Items/Str/DT_ItemTable.DT_ItemTable"))
    (if (and (> _returnvalue_3 0) (<= _returnvalue_3 (Utilities|Array|Length _outrownames)))
      (bind _outrownames_2 (DataTable|GetDataTableRowNames "/Game/Blueprints/Items/Str/DT_ItemTable.DT_ItemTable"))
      (bind _returnvalue_4 (Utilities|GetDataTableRow "/Game/Blueprints/Items/Str/DT_ItemTable.DT_ItemTable" (Utilities|Array|Get(acopy) _outrownames_2 (- _returnvalue_3 1)))
        (:then
          (CallFunction|SetItem _returnvalue_4)
          (Development|PrintText (Utilities|Text|ToText(String) (Utilities|String|Append "Got Item: " (.Name (Utilities|Struct|BreakStr_Item _returnvalue_4))))))
        (:RowNotFound
          (Development|PrintText "Invalid Item?"))))))

(fn ConstructionScript)

(fn Suspensions
  (params (Wheels :type Scene%20Component%20Object%20Reference) (BoneName :type Name))
  (bind _returnvalue (Transformation|GetWorldLocation Wheels))
  (bind _outhit (Collision|LineTraceByChannel _returnvalue (+ _returnvalue (* (Math|Vector|GetUpVector Wheels) (Variables|Default|GetDistance))) "TraceTypeQuery1" false 0 "None"))
  (if (.bBlockingHit (Collision|BreakHitResult _outhit))
    (Class|PrimitiveComponent|AddForceatLocation (Variables|Default|GetBox) (* (- 1.0 (Math|Float|NormalizetoRange (.Distance (Collision|BreakHitResult _outhit)) 0.0 (Math|Float|Absolute(Float) (.Z (Math|Vector|BreakVector "0.000000,0.000000,-30.000000"))))) (Math|Vector|GetUnitDirection(Vector) (.TraceEnd (Collision|BreakHitResult _outhit)) (.TraceStart (Collision|BreakHitResult _outhit))) 97500) (Transformation|GetWorldLocation Wheels) BoneName)
    (Class|PrimitiveComponent|AddForceatLocation (Variables|Default|GetBox) (* (Math|Vector|GetForwardVector (Variables|Default|GetBox)) (Variables|/Game/Vehicles/DA_EngineStats.DA_EngineStats_C|GetMaxSpeed_DA (Variables|Default|GetEngineDataAsset)) (Variables|Default|GetAccelerationInput) 6e+01 (Variables|Default|GetSpeedMod)) (Transformation|GetWorldLocation Wheels) "None")
    (return (.bBlockingHit (Collision|BreakHitResult _outhit)))))

(fn SwitchGameplayTypes
  (if (== (Variables|Default|GetVehicle%20State) 0)
    (Physics|SetEnableGravity (Variables|Default|GetBox) false)
    (Variables|Default|SetVehicle%20State "NewEnumerator1")
    (else
      (Physics|SetEnableGravity (Variables|Default|GetBox) true)
      (Variables|Default|SetVehicle%20State "NewEnumerator0"))))

(fn FlightControls
  (Physics|AddForce (Variables|Default|GetBox) (* (Math|Vector|GetForwardVector (Variables|Default|GetBox)) 1500000 (Variables|Default|GetAccelerationInput)) "None" false))

(fn CalculateAcceleration
  (Variables|Default|SetAccelleration (Math|Float|Lerp 0.0 (Variables|/Game/Vehicles/DA_EngineStats.DA_EngineStats_C|GetAcceleration_DA (Variables|Default|GetEngineDataAsset)) (Variables|Default|GetAccelerationInput)))
  (Variables|Default|SetAccelerationInput (Math|Interpolation|FInterpTo (Variables|Default|GetAccelerationInput) 0.0 (Utilities|Time|GetWorldDeltaSeconds) 0.3))
  (bind _asgi_racing_manager (Utilities|Casting|CastToGI_RacingManager (Game|GetGameInstance)))
  (Default|SetEventParameter _asgi_racing_manager (Variables|/Game/Blueprints/GI_RacingManager.GI_RacingManager_C|GetCurrentEngine _asgi_racing_manager) (Variables|/Game/Blueprints/GI_RacingManager.GI_RacingManager_C|GetEngineValue _asgi_racing_manager) 0.0))

(fn Drift
  (params (DriftStat :type Float%20%28double-precision%29) (Release :type Boolean) (SteerFactor :type Float%20%28double-precision%29))
  (Variables|Default|SetIsDrifting true)
  (if (>= SteerFactor 0.0)
    (Variables|Default|SetDriftFact (Math|Float|Lerp 0.0 3.5 SteerFactor))
    (else
      (Variables|Default|SetDriftFact (Math|Float|Lerp 0.0 -3.5 SteerFactor))))
  (Utilities|Time|SetTimerbyFunctionName 0 "Drift Level" 1.0 (Variables|Default|GetIsDrifting)))

(fn DriftBoost
  (params (BoostLevel :type Byte))
  (bind _returnvalue (Math|Conversions|ToFloat(Byte) BoostLevel))
  (bind _returnvalue_2 (Math|Float|Clamp(Float) _returnvalue 1.0 3.0))
  (if (>= BoostLevel 1)
    (CallFunction|Boost 1.5 _returnvalue_2)
    (Development|PrintString (Utilities|String|ToString(Float) _returnvalue_2))))

(fn Boost
  (params (SpeedMod :type Float%20%28double-precision%29) (Time :type Float%20%28single-precision%29))
  (Variables|Default|SetSpeedMod SpeedMod)
  (Utilities|Time|SetTimerbyFunctionName 0 "ResetSpeed" Time)
  ;[1 1 1] SFX
  (bind _asgi_racing_manager (Utilities|Casting|CastToGI_RacingManager (Game|GetGameInstance)))
  (Default|PlayOneShot _asgi_racing_manager "/Game/FMOD/Events/SFX/VEHICLE/Boost.Boost" "NewEnumerator2")
  (Components|Activation|Activate (Variables|Default|GetSpeedVFX) false))

(fn ResetSpeed
  (Variables|Default|SetSpeedMod 1.0)
  (Components|Activation|Deactivate (Variables|Default|GetSpeedVFX)))

(fn DriftLevel
  (if (>= 3 (Variables|Default|GetBoost%20Level))
    (Variables|Default|SetBoost%20Level (+ (Variables|Default|GetBoost%20Level) 1))))

(fn RotationBias
  (params (DeltaTime :type Float%20%28double-precision%29))
  (bind _returnvalue (Transformation|GetActorRotation))
  (bind _returnvalue_2 (Math|Interpolation|RInterpTo (Math|Rotator|MakeRotator (.roll _returnvalue) (.pitch _returnvalue) (.yaw _returnvalue)) (Math|Rotator|MakeRotator 0.0 0.0 (.yaw _returnvalue)) DeltaTime 0.5))
  (Transformation|SetRelativeRotation (Variables|Default|GetBox) _returnvalue_2 false false)
  (Development|PrintString (Utilities|String|ToString(Rotator) _returnvalue_2)))

(fn GetTrackProgression
  (bind _returnvalue (Transformation|GetVelocity))
  (bind _returnvalue_2 (Transformation|GetActorLocation))
  (bind _track (Variables|Default|GetTrack))
  (bind _returnvalue_3 (Math|Vector|Normalize _returnvalue))
  (bind _spline (Variables|/Game/Placeables/Laps/BP_TrackSpline.BP_TrackSpline_C|GetSpline _track))
  (bind _returnvalue_4 (Spline|FindLocationClosesttoWorldLocation _spline _returnvalue_2 "World"))
  (bind _returnvalue_5 (Spline|FindDirectionClosesttoWorldLocation _spline _returnvalue_4 "World"))
  (bind _returnvalue_6 (Math|Vector|DotProduct _returnvalue_5 _returnvalue_3))
  (bind _returnvalue_7 (> _returnvalue_6 0.0))
  (Development|PrintString (Utilities|String|SelectString "Forward" "Backwards" _returnvalue_7) true true "(R=0.000000,G=0.660000,B=1.000000,A=1.000000)" 0.0)
  (return _returnvalue_7))

(fn SetItem
  (params (Item :type Str%20Item%20Structure))
  (Default|SetNewItem (Variables|Default|GetBP_Item) Item))

(fn Damage
  (params (Damage :type Integer))
  (Development|PrintString (Utilities|String|Append "Damage Applied: " (Utilities|String|ToString(Integer) Damage)))
  ;[1 1 1] 1: EMP damage 2: spinout 3(default): full stop
  (switch int Damage
    (:Default
      (CallFunction|Damage 3))
    (:1
      (CallFunction|Damage 2)
      (Variables|Default|SetSpeedMod 0.45)
      (Variables|Default|SetAccelleration (* 0.65 (Variables|Default|GetAccelleration)))
      (Utilities|Time|SetTimerbyFunctionName 0 "ResetSpeed" 1e+01))
    (:2
      (Variables|Default|SetSpeedMod 0.15)
      (Variables|Default|SetAccelleration (* 0.3 (Variables|Default|GetAccelleration)))
      (Utilities|Time|SetTimerbyFunctionName 0 "ResetSpeed" 1.0))
    (:3
      (Variables|Default|SetSpeedMod 0.005)
      (Variables|Default|SetAccelleration (* 0.1 (Variables|Default|GetAccelleration)))
      (Utilities|Time|SetTimerbyFunctionName 0 "ResetSpeed" 1.5)
      (Utilities|Time|SetTimerbyFunctionName 0 "ResetAcceleration" 1.5))))

(fn Autopilot
  (bind _returnvalue (Transformation|GetActorLocation))
  (bind _track (Variables|Default|GetTrack))
  (bind _spline (Variables|/Game/Placeables/Laps/BP_TrackSpline.BP_TrackSpline_C|GetSpline _track))
  (if (> (Math|Float|Absolute(Float) (Math|Vector|DotProduct (Transformation|GetActorRightVector) (Math|Vector|GetVectorArrayAverage (Utilities|Array|MakeArray (Math|Vector|GetUnitDirection(Vector) _returnvalue (Class|SplineComponent|GetLocationatSplineInputKey _spline (+ (Class|SplineComponent|FindInputKeyClosesttoWorldLocation _spline _returnvalue) (* (Variables|Default|GetAccelerationInput) 0.7)) "World")) (Math|Vector|Normalize (Class|SplineComponent|GetTangentatSplineInputKey _spline (+ (Class|SplineComponent|FindInputKeyClosesttoWorldLocation _spline _returnvalue) (* (Variables|Default|GetAccelerationInput) 0.7)) "World")))))) 0.4)
    (Variables|Default|SetAccelerationInput (Math|Float|Clamp(Float) (- 0.5 (Math|Float|Absolute(Float) (Math|Vector|DotProduct (Transformation|GetActorRightVector) (Math|Vector|GetVectorArrayAverage (Utilities|Array|MakeArray (Math|Vector|GetUnitDirection(Vector) _returnvalue (Class|SplineComponent|GetLocationatSplineInputKey _spline (+ (Class|SplineComponent|FindInputKeyClosesttoWorldLocation _spline _returnvalue) (* (Variables|Default|GetAccelerationInput) 0.7)) "World")) (Math|Vector|Normalize (Class|SplineComponent|GetTangentatSplineInputKey _spline (+ (Class|SplineComponent|FindInputKeyClosesttoWorldLocation _spline _returnvalue) (* (Variables|Default|GetAccelerationInput) 0.7)) "World"))))))) 0.2 0.5))
    (else
      (Variables|Default|SetAccelerationInput 0.5)))
  (if (Utilities|Enum|Equal(Enum) (Variables|Default|GetVehicle%20State) "NewEnumerator0")
    (Class|PrimitiveComponent|AddTorqueinRadians (Variables|Default|GetBox) (Math|Vector|MakeVector 0.0 0.0 (* (* (.X (Math|Vector2D|BreakVector2D (Math|Vector2D|MakeVector2D (* (Math|Vector|DotProduct (Transformation|GetActorRightVector) (Math|Vector|GetVectorArrayAverage (Utilities|Array|MakeArray (Math|Vector|GetUnitDirection(Vector) _returnvalue (Class|SplineComponent|GetLocationatSplineInputKey _spline (+ (Class|SplineComponent|FindInputKeyClosesttoWorldLocation _spline _returnvalue) (* (Variables|Default|GetAccelerationInput) 0.7)) "World")) (Math|Vector|Normalize (Class|SplineComponent|GetTangentatSplineInputKey _spline (+ (Class|SplineComponent|FindInputKeyClosesttoWorldLocation _spline _returnvalue) (* (Variables|Default|GetAccelerationInput) 0.7)) "World"))))) 5.0) (* (Math|Vector|DotProduct (Math|Vector|GetVectorArrayAverage (Utilities|Array|MakeArray (Math|Vector|GetUnitDirection(Vector) _returnvalue (Class|SplineComponent|GetLocationatSplineInputKey _spline (+ (Class|SplineComponent|FindInputKeyClosesttoWorldLocation _spline _returnvalue) (* (Variables|Default|GetAccelerationInput) 0.7)) "World")) (Math|Vector|Normalize (Class|SplineComponent|GetTangentatSplineInputKey _spline (+ (Class|SplineComponent|FindInputKeyClosesttoWorldLocation _spline _returnvalue) (* (Variables|Default|GetAccelerationInput) 0.7)) "World")))) (Transformation|GetActorUpVector)) 5.0)))) (Variables|Default|GetHandling) (Variables|Default|GetAccelerationInput)) (Variables|Default|GetDriftFact))) "None" false)
    (else
      (Transformation|AddLocalRotation (Variables|Default|GetBox) (Math|Rotator|MakeRotator 0.0 (Math|Float|Lerp 0.0 (* (.Y (Math|Vector2D|BreakVector2D (Math|Vector2D|MakeVector2D (* (Math|Vector|DotProduct (Transformation|GetActorRightVector) (Math|Vector|GetVectorArrayAverage (Utilities|Array|MakeArray (Math|Vector|GetUnitDirection(Vector) _returnvalue (Class|SplineComponent|GetLocationatSplineInputKey _spline (+ (Class|SplineComponent|FindInputKeyClosesttoWorldLocation _spline _returnvalue) (* (Variables|Default|GetAccelerationInput) 0.7)) "World")) (Math|Vector|Normalize (Class|SplineComponent|GetTangentatSplineInputKey _spline (+ (Class|SplineComponent|FindInputKeyClosesttoWorldLocation _spline _returnvalue) (* (Variables|Default|GetAccelerationInput) 0.7)) "World"))))) 5.0) (* (Math|Vector|DotProduct (Math|Vector|GetVectorArrayAverage (Utilities|Array|MakeArray (Math|Vector|GetUnitDirection(Vector) _returnvalue (Class|SplineComponent|GetLocationatSplineInputKey _spline (+ (Class|SplineComponent|FindInputKeyClosesttoWorldLocation _spline _returnvalue) (* (Variables|Default|GetAccelerationInput) 0.7)) "World")) (Math|Vector|Normalize (Class|SplineComponent|GetTangentatSplineInputKey _spline (+ (Class|SplineComponent|FindInputKeyClosesttoWorldLocation _spline _returnvalue) (* (Variables|Default|GetAccelerationInput) 0.7)) "World")))) (Transformation|GetActorUpVector)) 5.0)))) (Variables|Default|GetHandlin_Air) (Variables|Default|GetAccelerationInput) (Variables|Default|GetInverted)) 0.5) (Math|Float|Lerp 0.0 (* (.X (Math|Vector2D|BreakVector2D (Math|Vector2D|MakeVector2D (* (Math|Vector|DotProduct (Transformation|GetActorRightVector) (Math|Vector|GetVectorArrayAverage (Utilities|Array|MakeArray (Math|Vector|GetUnitDirection(Vector) _returnvalue (Class|SplineComponent|GetLocationatSplineInputKey _spline (+ (Class|SplineComponent|FindInputKeyClosesttoWorldLocation _spline _returnvalue) (* (Variables|Default|GetAccelerationInput) 0.7)) "World")) (Math|Vector|Normalize (Class|SplineComponent|GetTangentatSplineInputKey _spline (+ (Class|SplineComponent|FindInputKeyClosesttoWorldLocation _spline _returnvalue) (* (Variables|Default|GetAccelerationInput) 0.7)) "World"))))) 5.0) (* (Math|Vector|DotProduct (Math|Vector|GetVectorArrayAverage (Utilities|Array|MakeArray (Math|Vector|GetUnitDirection(Vector) _returnvalue (Class|SplineComponent|GetLocationatSplineInputKey _spline (+ (Class|SplineComponent|FindInputKeyClosesttoWorldLocation _spline _returnvalue) (* (Variables|Default|GetAccelerationInput) 0.7)) "World")) (Math|Vector|Normalize (Class|SplineComponent|GetTangentatSplineInputKey _spline (+ (Class|SplineComponent|FindInputKeyClosesttoWorldLocation _spline _returnvalue) (* (Variables|Default|GetAccelerationInput) 0.7)) "World")))) (Transformation|GetActorUpVector)) 5.0)))) (Variables|Default|GetHandlin_Air) 0.55) 0.5)) false false))))

(fn AutopilotToggle
  (if (Variables|Default|GetIsAutopilot)
    (Variables|Default|SetIsAutopilot false)
    (Variables|Default|SetCanDrive true)
    (Default|DecrementItemUse (Variables|Default|GetBP_Item))
    (Development|PrintText "autopilot toggle off")
    (else
      (Variables|Default|SetIsAutopilot true)
      (Variables|Default|SetCanDrive false)
      (Utilities|Time|SetTimerbyFunctionName 0 "AutopilotToggle" 12.0)
      (Development|PrintText "autopilot toggle on"))))

(fn BindSuspensions
  (params (DeltaTime :type Float%20%28double-precision%29))
  (bind _box (Variables|Default|GetBox))
  (bind _touchingfloor (CallFunction|Suspensions (Variables|Default|GetFrontWheel_L) "DEF-Wheel_Ft_L"))
  (bind _touchingfloor_2 (CallFunction|Suspensions (Variables|Default|GetFrontWheel_R) "DEF-Wheel_Ft_R"))
  (bind _touchingfloor_3 (CallFunction|Suspensions (Variables|Default|GetRearWheel_L) "DEF-Wheel_Bk_L"))
  (bind _touchingfloor_4 (CallFunction|Suspensions (Variables|Default|GetRearWheel_R) "DEF-Wheel_Bk_R"))
  (if (Math|Boolean|ANDBoolean _touchingfloor _touchingfloor_2 _touchingfloor_3 _touchingfloor_4)
    (Variables|Default|SetIsOnGround true)
    (Physics|SetEnableGravity (Variables|Default|GetBox) false)
    (else
      (Variables|Default|SetIsOnGround false)
      (Physics|SetEnableGravity (Variables|Default|GetBox) true)
      (Class|PrimitiveComponent|AddForceatLocation (Variables|Default|GetBox) (+ (* (Math|Vector|GetForwardVector _box) (Variables|Default|GetMax_Speed) (Variables|Default|GetAccelerationInput) 6e+01 (Variables|Default|GetSpeedMod)) "0.000000,0.000000,-360000.000000") (Transformation|GetWorldLocation _box) "None")
      (CallFunction|RotationBias DeltaTime))))

(fn CollisionPush
  (params (Force :type Vector))
  (Physics|AddForce (Variables|Default|GetBox) Force "None" false))