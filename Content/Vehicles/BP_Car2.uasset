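; Player-driven physics car that moves a Box body with forces and torques, with ground and flight states.
; On the ground, four wheel line traces each apply spring suspension and forward drive when they hit.
; In flight, a constant-scale thrust replaces suspension, scaled by an eased throttle that also affects steering torque and drift.
; The gravity-toggling state switch is unwired, and Boost is an empty stub.
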(event `self.ReceiveBeginPlay`
  ;[0.1928 1 0] Casting Player Controller
  (bind _asplayer_controller (cast `PlayerController` (`self.GetController`)))
  (message `EnhancedInputSubsystemInterface.AddMappingContext` (pcsubsystem `EnhancedInputLocalPlayerSubsystem` _asplayer_controller) "/Game/InputMapping/IA_Player.IA_Player" 0 (struct)))

(event `self.ReceiveActorBeginOverlap`
  (params (OtherActor :type "Actor Object Reference")))

(event `EnhancedInput|/Game/InputMapping/InputActions/IA_Accelerate`
  (params (ActionValue :type Boolean) (ElapsedSeconds :type "Float (double-precision)") (TriggeredSeconds :type "Float (double-precision)") (InputAction :type "InputAction Object Reference" :default "/Game/InputMapping/InputActions/IA_Accelerate.IA_Accelerate"))
  (:`Triggered`
    (set `self.AccelerationInput` (`KismetMathLibrary.FInterpTo` (`self.AccelerationInput`) 1.0 (`GameplayStatics.GetWorldDeltaSeconds`) 0.2))))

(event `EnhancedInput|/Game/InputMapping/InputActions/IA_Drift`
  (params (ActionValue :type Boolean) (ElapsedSeconds :type "Float (double-precision)") (TriggeredSeconds :type "Float (double-precision)") (InputAction :type "InputAction Object Reference" :default "/Game/InputMapping/InputActions/IA_Drift.IA_Drift"))
  (:`Triggered`
    (`self.Drift` (* (`KismetMathLibrary.BreakVector2D` (stale `EnhancedInput|/Game/InputMapping/InputActions/IA_Steer` ActionValue)) (`self.Handling`) (`self.AccelerationInput`)))
    (`KismetSystemLibrary.PrintString` "Drifting")))

(event `EnhancedInput|/Game/InputMapping/InputActions/IA_Steer`
  (params (ActionValue :type "Vector2D Structure") (ElapsedSeconds :type "Float (double-precision)") (TriggeredSeconds :type "Float (double-precision)") (InputAction :type "InputAction Object Reference" :default "/Game/InputMapping/InputActions/IA_Steer.IA_Steer"))
  (bind (_x _y) (`KismetMathLibrary.BreakVector2D` ActionValue))
  (:`Triggered`
    (if (`|EnumEquality` (`self.Vehicle State`) "NewEnumerator0")
      (`PrimitiveComponent.AddTorqueInRadians` (`self.Box`) (`KismetMathLibrary.MakeVector` 0.0 0.0 (* _x (`self.Handling`) (`self.AccelerationInput`))) "None" false)
      (else
        (`PrimitiveComponent.AddTorqueInRadians` (`self.Box`) (`KismetMathLibrary.MakeVector` 0.0 (* _y (`self.Handlin_Air`) (`self.AccelerationInput`)) (* _x (`self.Handlin_Air`))) "None" false)))))

(event `self.ReceiveTick`
  (params (DeltaSeconds :type "Float (single-precision)"))
  (if (`|EnumEquality` (`self.Vehicle State`) "NewEnumerator0")
    ;[0.763 0.09722 1] Set Suspensions on Vehicel
    (`self.Suspensions` (`self.FrontWheel_L`))
    (`self.Suspensions` (`self.FrontWheel_R`))
    (`self.Suspensions` (`self.RearWheel_L`))
    (`self.Suspensions` (`self.RearWheel_R`))
    (`self.Calculate Acceleration`)
    (else
      (`self.Flight_Controls`)
      (`self.Calculate Acceleration`))))

(fn `Boost`)

(fn `Calculate Acceleration`
  (set `self.Accelleration` (`KismetMathLibrary.Lerp` 0.0 3000.0 (`self.AccelerationInput`)))
  (set `self.AccelerationInput` (`KismetMathLibrary.FInterpTo` (`self.AccelerationInput`) 0.0 (`GameplayStatics.GetWorldDeltaSeconds`) 0.3)))

(fn `Drift`
  (params (HandlingInput :type "Float (double-precision)"))
  (if (not (> (`KismetMathLibrary.Abs` HandlingInput) 0.5))
    (`PrimitiveComponent.AddForce` (`self.Box`) (`KismetMathLibrary.MakeVector` (* HandlingInput (* (`self.Handling`) 2.0))) "None" false)
    (`KismetSystemLibrary.PrintString` (`KismetStringLibrary.Conv_VectorToString` (`KismetMathLibrary.Conv_DoubleToVector` HandlingInput)))))

(fn `Flight_Controls`
  (`PrimitiveComponent.AddForce` (`self.Box`) (* (`SceneComponent.GetForwardVector` (`self.Box`)) 750000 (`self.AccelerationInput`)) "None" false))

(fn `Suspensions`
  (params (Wheels :type "SceneComponent Object Reference"))
  (bind _returnvalue (`SceneComponent.K2_GetComponentLocation` Wheels))
  (bind _outhit (`KismetSystemLibrary.LineTraceSingle` :`Start` _returnvalue :`End` (+ _returnvalue (* (`SceneComponent.GetUpVector` Wheels) (`self.Distance`))) :`TraceChannel` "TraceTypeQuery1" :`DrawDebugType` "ForOneFrame"))
  (bind (_bblockinghit _binitialoverlap _time _distance _location _impactpoint _normal _impactnormal _physmat _hitactor _hitcomponent _hitbonename _bonename _hititem _elementindex _faceindex _tracestart _traceend) (`GameplayStatics.BreakHitResult` _outhit))
  (if _bblockinghit
    (`PrimitiveComponent.AddForceAtLocation` (`self.Box`) (* (- 1.0 (`KismetMathLibrary.NormalizeToRange` _distance 0.0 (`KismetMathLibrary.Abs` (.z (0.0 0.0 -30.0))))) (`KismetMathLibrary.GetDirectionUnitVector` _traceend _tracestart) 92000) (`SceneComponent.K2_GetComponentLocation` (`local.Wheels`)) "None")
    (`PrimitiveComponent.AddForceAtLocation` (`self.Box`) (* (`SceneComponent.GetForwardVector` (`self.Box`)) (`self.Max_Speed`) (`self.AccelerationInput`) 60.0) (`SceneComponent.K2_GetComponentLocation` (`local.Wheels`)) "None")))

(fn `SwitchGameplayTypes`
  (if (== (`self.Vehicle State`) 0)
    (`PrimitiveComponent.SetEnableGravity` (`self.Box`) false)
    (set `self.Vehicle State` "NewEnumerator1")
    (else
      (`PrimitiveComponent.SetEnableGravity` (`self.Box`) true)
      (set `self.Vehicle State` "NewEnumerator0"))))

(fn `UserConstructionScript`)