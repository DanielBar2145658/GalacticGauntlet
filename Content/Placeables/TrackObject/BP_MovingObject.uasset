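; Actor component that moves its owner in a continuous loop along a spline, facing the spline tangent.
; While active, Tick advances a spline input key by delta time and a speed modifier, wrapping past the point count, so speed follows point spacing rather than distance.
; BeginLoop starts movement on the assigned spline.
; BeginLoopGenerateSpline first spawns a given class at the owner's transform and uses its spline component.
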(event `self.ReceiveTick`
  (params (DeltaSeconds :type "Float (single-precision)"))
  (bind _returnvalue (`SplineComponent.GetNumberOfSplinePoints` (`self.Spline`)))
  (bind _returnvalue_2 (+ (* DeltaSeconds (`self.SpeedMod`)) (`self.CurrentSplineKey`)))
  (if (`self.Active`)
    (if (> _returnvalue_2 _returnvalue)
      (bind _output_get (set `self.CurrentSplineKey` (- _returnvalue_2 _returnvalue)))
      (`self.SetLocationOnSpline` _output_get)
      (else
        (bind _output_get_2 (set `self.CurrentSplineKey` _returnvalue_2))
        (`self.SetLocationOnSpline` _output_get_2)))))

(fn `BeginLoop`
  (`/Engine/EditorBlueprintResources/StandardMacros.IsValid` (`self.Spline`)
    (:`Is Valid`
      (`self.SetLocationOnSpline` 0.0)
      (set `self.Active` true))
    (:`Is Not Valid`
      (`KismetSystemLibrary.PrintString` "moving object has no spline!"))))

(fn `BeginLoopGenerateSpline`
  (params (Class :type "Actor Class Reference"))
  (bind (_returnvalue_location _returnvalue_rotation) (`KismetMathLibrary.BreakTransform` (`Actor.GetTransform` (`self.GetOwner`))))
  (bind _returnvalue (`|SpawnActorFromClass` Class (`KismetMathLibrary.MakeTransform` _returnvalue_location _returnvalue_rotation) "Undefined" "MultiplyWithRoot" null null))
  (bind _returnvalue_2 (`Actor.GetComponentByClass` _returnvalue "/Script/Engine.SplineComponent"))
  (`/Engine/EditorBlueprintResources/StandardMacros.IsValid` _returnvalue_2
    (:`Is Valid`
      (set `self.Spline` _returnvalue_2)
      (`self.BeginLoop`))
    (:`Is Not Valid`
      (`KismetSystemLibrary.PrintString` "spline cannot be generated from class"))))

(fn `SetLocationOnSpline`
  (params (Key :type "Float (double-precision)"))
  (bind _spline (`self.Spline`))
  (`Actor.K2_SetActorTransform` (`self.GetOwner`) (`KismetMathLibrary.MakeTransform` (`SplineComponent.GetLocationAtSplineInputKey` _spline Key "World") (`KismetMathLibrary.MakeRotFromX` (`SplineComponent.GetTangentAtSplineInputKey` _spline Key "World"))) false false))