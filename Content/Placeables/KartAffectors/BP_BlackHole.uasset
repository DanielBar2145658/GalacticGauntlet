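; BP_BlackHole is a placeable kart affector that drags cars inside its trigger toward its center while swirling them around it.
; Each tick it moves every overlapping BP_Car by a pull along the direction to the hole, plus a tangential offset from crossing the car's up vector with that direction.
; BaseSpeed scales both motions and OrbitFactor weights the swirl, applied as unswept world offsets rather than physics forces.
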(event `self.ReceiveTick`
  (params (DeltaSeconds :type "Float (single-precision)"))
  (bind _returnvalue (* (`self.BaseSpeed`) DeltaSeconds))
  (for _array_element (`PrimitiveComponent.GetOverlappingActors` (`self.Trigger`) "/Game/Vehicles/BP_Car.BP_Car_C")
    (bind _returnvalue_2 (`KismetMathLibrary.GetDirectionUnitVector` (`self.K2_GetActorLocation` _array_element) (`self.K2_GetActorLocation`)))
    (`self.K2_AddActorWorldOffset` _array_element (+ (* (`KismetMathLibrary.Cross_VectorVector` (`self.GetActorUpVector` _array_element) _returnvalue_2) _returnvalue (`self.OrbitFactor`)) (* _returnvalue_2 _returnvalue)) false false)))

(fn `UserConstructionScript`)